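; LED indicator that shows the progress of BP_Lever as a red, two-orange and green light sequence.
; While State is true, Tick polls LeverState and sets material color and glow: red at the start, green at the end, which also clears State.
; In between, IsHolding plays or reverses a Timeline that fades the oranges, with a delayed red switch-off.
; Two cross-resetting DoOnce nodes keep Tick from retriggering the Timeline.
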(event EventTick
  (params (DeltaSeconds :type Float%20%28single-precision%29))
  (bind _led3 (Variables|Default|GetLED3))
  (bind _led1 (Variables|Default|GetLED1))
  (bind _led2 (Variables|Default|GetLED2))
  (bind _led3_2 (Variables|Default|GetLED3))
  (bind _led5 (Variables|Default|GetLED5))
  (bind _led1_2 (Variables|Default|GetLED1))
  (bind _led2_2 (Variables|Default|GetLED2))
  (bind _led5_2 (Variables|Default|GetLED5))
  (bind _led1_3 (Variables|Default|GetLED1))
  (bind _led2_3 (Variables|Default|GetLED2))
  (bind _led3_3 (Variables|Default|GetLED3))
  (if (Variables|Default|GetState)
    (bind _returnvalue (Actor|GetActorOfClass "/Game/Blueprints/BP_Lever.BP_Lever_C"))
    (switch int (Variables|/Game/Blueprints/BP_Lever.BP_Lever_C|GetLeverState _returnvalue)
      (:Default
        (Rendering|Material|SetScalarParameterValueonMaterials (Variables|Default|GetLED2) "light" 0.0)
        (Rendering|Material|SetScalarParameterValueonMaterials (Variables|Default|GetLED1) "light" 2e+01))
      (:0
        ;[0.15 0.15 0.15 0.5] red led1
        (Rendering|Material|SetColorParameterValueonMaterials _led1_3 "color" "(R=1.000000,G=0.000000,B=0.000000,A=1.000000)")
        (Rendering|Material|SetScalarParameterValueonMaterials _led1_3 "light" 2e+01)
        ;[0.15 0.15 0.15 0.5] orange1 led2
        (Rendering|Material|SetColorParameterValueonMaterials _led2_3 "color" "(R=1.000000,G=0.296138,B=0.000000,A=1.000000)")
        (Rendering|Material|SetScalarParameterValueonMaterials _led2_3 "light" 0.0)
        ;[0.15 0.15 0.15 0.5] orange2 led3
        (Rendering|Material|SetColorParameterValueonMaterials _led3_3 "color" "(R=1.000000,G=0.296138,B=0.000000,A=1.000000)")
        (Rendering|Material|SetScalarParameterValueonMaterials _led3_3 "light" 0.0)
        ;[0.15 0.15 0.15 0.5] green led5
        (Rendering|Material|SetColorParameterValueonMaterials _led5_2 "color" "(R=0.000000,G=1.000000,B=0.000000,A=1.000000)")
        (Rendering|Material|SetScalarParameterValueonMaterials _led5_2 "light" 0.0)
        (Utilities|FlowControl|Sequence
          (:then_0
            (goto _label Reset))
          (:then_1
            (bind (_direction _新建轨道_0 _新建轨道_1) (Timeline|时间轴 Stop)
              (:Update
                (Utilities|FlowControl|Sequence
                  (:then_0
                    ;[0.15 0.15 0.15 0.5] orange1 led2
                    (Rendering|Material|SetColorParameterValueonMaterials _led2_2 "color" "(R=1.000000,G=0.296138,B=0.000000,A=1.000000)")
                    (Rendering|Material|SetScalarParameterValueonMaterials _led2_2 "light" _新建轨道_0)
                    ;[0.15 0.15 0.15 0.5] orange2 led3
                    (Rendering|Material|SetColorParameterValueonMaterials _led3 "color" "(R=1.000000,G=0.296138,B=0.000000,A=1.000000)")
                    (Rendering|Material|SetScalarParameterValueonMaterials _led3 "light" _新建轨道_1))
                  (:then_1
                    ;[0.15 0.15 0.15 0.5] red led1
                    (Utilities|FlowControl|Delay 1.95)
                    (Rendering|Material|SetColorParameterValueonMaterials _led1_2 "color" "(R=1.000000,G=0.000000,B=0.000000,A=1.000000)")
                    (Rendering|Material|SetScalarParameterValueonMaterials _led1_2 "light" 0.0))))))
          (:then_2
            (goto _label_2 Reset))))
      (:1
        (bind _returnvalue_2 (Actor|GetActorOfClass "/Game/Blueprints/BP_Lever.BP_Lever_C"))
        (if (Variables|/Game/Blueprints/BP_Lever.BP_Lever_C|GetisHolding _returnvalue_2)
          (Utilities|FlowControl|DoOnce false :!label _label
            (:Completed
              (Utilities|FlowControl|Sequence
                (:then_0
                  (Timeline|时间轴 Play))
                (:then_1
                  (goto _label_2 Reset)))))
          (else
            (Utilities|FlowControl|DoOnce false :!label _label_2
              (:Completed
                (Utilities|FlowControl|Sequence
                  (:then_0
                    (Timeline|时间轴 Reverse))
                  (:then_1
                    (goto _label Reset))))))))
      (:2
        ;[0.15 0.15 0.15 0.5] red led1
        (Rendering|Material|SetColorParameterValueonMaterials _led1 "color" "(R=1.000000,G=0.000000,B=0.000000,A=1.000000)")
        (Rendering|Material|SetScalarParameterValueonMaterials _led1 "light" 0.0)
        ;[0.15 0.15 0.15 0.5] orange1 led2
        (Rendering|Material|SetColorParameterValueonMaterials _led2 "color" "(R=1.000000,G=0.296138,B=0.000000,A=1.000000)")
        (Rendering|Material|SetScalarParameterValueonMaterials _led2 "light" 0.0)
        ;[0.15 0.15 0.15 0.5] orange2 led3
        (Rendering|Material|SetColorParameterValueonMaterials _led3_2 "color" "(R=1.000000,G=0.296138,B=0.000000,A=1.000000)")
        (Rendering|Material|SetScalarParameterValueonMaterials _led3_2 "light" 0.0)
        ;[0.15 0.15 0.15 0.5] green led5
        (Rendering|Material|SetColorParameterValueonMaterials _led5 "color" "(R=0.000000,G=1.000000,B=0.000000,A=1.000000)")
        (Rendering|Material|SetScalarParameterValueonMaterials _led5 "light" 2e+01)
        (Utilities|FlowControl|Sequence
          (:then_0
            (Timeline|时间轴 Stop))
          (:then_1
            (Variables|Default|SetState false)))))))

(fn ConstructionScript)