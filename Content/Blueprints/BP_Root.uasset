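; BP_Root is an interactable root obstacle that the player cuts away with a knife to clear it from a parent mechanic.
; On interact, if the first-person character holds a knife and the parent implements BPI_RootsAttachment, it notifies that parent, clears the focused actor and destroys itself.
; Focus events toggle an outline overlay material and a widget, and gaining focus triggers the crosshair's knife interaction hint.
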(event EventInteract
  (bind _parentmechanic (Variables|Default|GetParentMechanic))
  (bind _asbp_first_person_character (Utilities|Casting|CastToBP_FirstPersonCharacter (Game|GetPlayerCharacter 0)))
  (if (Variables|/Game/FirstPerson/Blueprints/BP_FirstPersonCharacter.BP_FirstPersonCharacter_C|GetisHoldingKnife _asbp_first_person_character)
    (Utilities|IsValid _parentmechanic
      (:Is%20Valid
        (if (Utilities|DoesObjectImplementInterface _parentmechanic "/Game/Blueprints/BPI_RootsAttachment.BPI_RootsAttachment_C")
          (Class|BPIRootsAttachment|RemoveRootsBool(Message) _parentmechanic)
          (Variables|/Game/FirstPerson/Blueprints/BP_FirstPersonCharacter.BP_FirstPersonCharacter_C|SetFocusedActor _asbp_first_person_character 0)
          (Actor|DestroyActor))))))

(event EventOnFocus
  ;[0.15 0.15 0.15 0.5] UI
  (Rendering|Material|SetOverlayMaterial (Variables|Default|GetRoot) "/Game/LevelPrototyping/Materials/M_InteractOutline.M_InteractOutline" :!class /Script/Engine.MeshComponent)
  (Rendering|SetVisibility (Variables|Default|GetWidget) true false)
  (bind _foundwidgets (Widget|GetAllWidgetsOfClass "/Game/UI/WBP_Crosshair.WBP_Crosshair_C" true))
  (Default|KnifeInteractHelp _foundwidgets))

(event EventNotonFocus
  ;[0.15 0.15 0.15 0.5] UI
  (Rendering|Material|SetOverlayMaterial (Variables|Default|GetRoot) 0 :!class /Script/Engine.MeshComponent)
  (Rendering|SetVisibility (Variables|Default|GetWidget) false false))

(fn ConstructionScript
  (|CallParentFunction))

(fn DestroyRoot
  (Actor|DestroyActor))