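; BP_LoadingWall is an actor that moves its Wall component straight up from where it starts.
; BeginPlay caches the start location and a target 1000 units above it.
; Tick calls Play on the WallMove timeline every frame, which lerps the wall between the two points.
; When the timeline finishes, the wall teleports back to its start location.
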(event Collision|EventActorBeginOverlap
  (params (OtherActor :type Actor%20Object%20Reference)))

(event EventBeginPlay
  (Variables|Default|SetStartingLocation (Transformation|GetWorldLocation (Variables|Default|GetWall)))
  (Variables|Default|SetTargetLocation (+ (Variables|Default|GetStartingLocation) "0.000000,0.000000,1000.000000")))

(event EventTick
  (params (DeltaSeconds :type Float%20%28single-precision%29))
  (bind _alpha (Timeline|WallMove Play)
    (:Update
      (Transformation|SetWorldLocation (Variables|Default|GetWall) (Math|Vector|Lerp(Vector) (Variables|Default|GetStartingLocation) (Variables|Default|GetTargetLocation) _alpha) false false))
    (:Finished
      (Transformation|SetWorldLocation (Variables|Default|GetWall) (Variables|Default|GetStartingLocation) false true))))

(fn ConstructionScript)