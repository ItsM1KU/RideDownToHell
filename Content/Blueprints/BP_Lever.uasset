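; Hold-to-pull lever that the first-person player works by mouse or interact while inside its trigger box.
; Pressing freezes movement and look; if BP_lightt's State is on, the view blends to a lever camera until release or completion.
; Tick polls LeverState to drive a rotation timeline, with DoOnce gates reversing an early release.
; Focus shows an outline and hold hint; elevator activation is present but unwired.
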(event OnComponentBeginOverlap(TriggerBox)
  (params (OverlappedComponent :type Primitive%20Component%20Object%20Reference) (OtherActor :type Actor%20Object%20Reference) (OtherComp :type Primitive%20Component%20Object%20Reference) (OtherBodyIndex :type Integer) (bFromSweep :type Boolean) (SweepResult :type Hit%20Result%20Structure%20%28by%20ref%29))
  ;[0.15 0.15 0.15 0.5] lever trigger
  (Variables|Default|SetisNearLever true))

(event OnComponentEndOverlap(TriggerBox)
  (params (OverlappedComponent :type Primitive%20Component%20Object%20Reference) (OtherActor :type Actor%20Object%20Reference) (OtherComp :type Primitive%20Component%20Object%20Reference) (OtherBodyIndex :type Integer))
  ;[0.15 0.15 0.15 0.5] lever trigger
  (Variables|Default|SetisNearLever false))

(event Custom|lever%20rotate
  ;[0.15 0.15 0.15 0.5] lever rotate
  (switch int (Variables|Default|GetLeverState)
    (:1
      (if (Variables|Default|GetisHolding)
        (Utilities|FlowControl|DoOnce false :!label _label
          (:Completed
            (Utilities|FlowControl|Sequence
              (:then_0
                (bind _新建轨道_0 (Timeline|时间轴 Play)
                  (:Update
                    (Transformation|SetRelativeRotation (Variables|Default|Getlever) (Math|Rotator|MakeRotator 0.0 (Math|Float|Lerp -4e+01 (Variables|Default|GetLeverPullAngle) _新建轨道_0) 0.0) false false))
                  (:Finished
                    (if (Variables|Default|GetisHolding)
                      (Variables|Default|SetLeverState 2)
                      (Utilities|FlowControl|Delay 1.0)
                      (bind _asbp_first_person_character (Utilities|Casting|CastToBP_FirstPersonCharacter (Game|GetPlayerCharacter 0)))
                      (Game|Player|SetViewTargetwithBlend (Game|GetPlayerController 0) _asbp_first_person_character 1.0 "VTBlend_Linear" 0.0 false)
                      (else
                        (Variables|Default|SetLeverState 0))))))
              (:then_1
                (goto _label_2 Reset)))))
        (else
          (Utilities|FlowControl|DoOnce false :!label _label_2
            (:Completed
              (Utilities|FlowControl|Sequence
                (:then_0
                  (Timeline|时间轴 Reverse))
                (:then_1
                  (goto _label Reset))))))))))

(event EventTick
  (params (DeltaSeconds :type Float%20%28single-precision%29))
  ;[0.15 0.15 0.15 0.5] test
  (Development|PrintString (Utilities|String|ToString(Integer) (Variables|Default|GetLeverState)))
  (CallFunction|LeverRotate))

(event EventMousePressed
  ;[0.15 0.15 0.15 0.5] camera & state
  (bind _asbp_first_person_character (Utilities|Casting|CastToBP_FirstPersonCharacter (Game|GetPlayerCharacter 0)))
  (Variables|Default|SetisHolding true)
  (if (Variables|Default|GetisNearLever)
    (Pawn|Components|CharacterMovement|SetMovementMode (Variables|/Script/Engine.Character|GetCharacterMovement _asbp_first_person_character) "MOVE_None" 0)
    (Input|SetIgnoreLookInput (Game|GetPlayerController 0) true)
    (Variables|Default|SetLeverState 1)
    (bind _returnvalue (Actor|GetActorOfClass "/Game/Blueprints/BP_lightt.BP_lightt_C"))
    (if (Variables|/Game/Blueprints/BP_lightt.BP_lightt_C|GetState _returnvalue)
      (bind _returnvalue_2 (Actor|GetActorOfClass "/Game/Blueprints/LeverCameraa.LeverCameraa_C"))
      (Game|Player|SetViewTargetwithBlend (Game|GetPlayerController 0) _returnvalue_2 1.0 "VTBlend_Linear" 0.0 false)
      (Timeline|时间轴_0 PlayFromStart
        (:Finished
          (Variables|Default|SetLeverState 2)
          (Utilities|FlowControl|Delay 1.0)
          (bind _asbp_first_person_character_2 (Utilities|Casting|CastToBP_FirstPersonCharacter (Game|GetPlayerCharacter 0)))
          (Game|Player|SetViewTargetwithBlend (Game|GetPlayerController 0) _asbp_first_person_character_2 1.0 "VTBlend_Linear" 0.0 false))))))

(event EventMouseReleased
  ;[0.15 0.15 0.15 0.5] camera & state
  (Pawn|Components|CharacterMovement|SetMovementMode (Variables|/Script/Engine.Character|GetCharacterMovement (stale EventMousePressed _asbp_first_person_character)) "MOVE_Walking" 0)
  (Input|SetIgnoreLookInput (Game|GetPlayerController 0) false)
  (bind _returnvalue (Actor|GetActorOfClass "/Game/Blueprints/BP_lightt.BP_lightt_C"))
  (if (Variables|/Game/Blueprints/BP_lightt.BP_lightt_C|GetState _returnvalue)
    (Variables|Default|SetisHolding false)
    (Utilities|FlowControl|Sequence
      (:then_0
        (Timeline|时间轴_0 Stop
          (:Finished
            (Variables|Default|SetLeverState 2)
            (Utilities|FlowControl|Delay 1.0)
            (bind _asbp_first_person_character (Utilities|Casting|CastToBP_FirstPersonCharacter (Game|GetPlayerCharacter 0)))
            (Game|Player|SetViewTargetwithBlend (Game|GetPlayerController 0) _asbp_first_person_character 1.0 "VTBlend_Linear" 0.0 false))))
      (:then_1
        (bind _asbp_first_person_character_2 (Utilities|Casting|CastToBP_FirstPersonCharacter (Game|GetPlayerCharacter 0)))
        (Game|Player|SetViewTargetwithBlend (Game|GetPlayerController 0) _asbp_first_person_character_2 1.0 "VTBlend_Linear" 0.0 false)))))

(event EventBeginPlay
  ;[0.15 0.15 0.15 0.5] input
  (Input|EnableInput (Game|GetPlayerController 0)))

(event EventOnFocus
  (Rendering|Material|SetOverlayMaterial (Variables|组件|GetLeverBase) "/Game/LevelPrototyping/Materials/M_InteractOutline.M_InteractOutline" :!class /Script/Engine.MeshComponent)
  (Rendering|SetVisibility (Variables|Default|GetW_Hold) true false)
  (bind _foundwidgets (Widget|GetAllWidgetsOfClass "/Game/UI/WBP_Crosshair.WBP_Crosshair_C" true))
  (Default|HoldInteractHelp _foundwidgets))

(event EventNotonFocus
  (Rendering|Material|SetOverlayMaterial (Variables|组件|GetLeverBase) 0 :!class /Script/Engine.MeshComponent)
  (Rendering|SetVisibility (Variables|Default|GetW_Hold) false false))

(event EventInteract
  ;[0.15 0.15 0.15 0.5] camera & state
  (bind _asbp_first_person_character (Utilities|Casting|CastToBP_FirstPersonCharacter (Game|GetPlayerCharacter 0)))
  (Variables|Default|SetisHolding true)
  (if (Variables|Default|GetisNearLever)
    (Pawn|Components|CharacterMovement|SetMovementMode (Variables|/Script/Engine.Character|GetCharacterMovement _asbp_first_person_character) "MOVE_None" 0)
    (Input|SetIgnoreLookInput (Game|GetPlayerController 0) true)
    (Variables|Default|SetLeverState 1)
    (bind _returnvalue (Actor|GetActorOfClass "/Game/Blueprints/BP_lightt.BP_lightt_C"))
    (if (Variables|/Game/Blueprints/BP_lightt.BP_lightt_C|GetState _returnvalue)
      (bind _returnvalue_2 (Actor|GetActorOfClass "/Game/Blueprints/LeverCameraa.LeverCameraa_C"))
      (Game|Player|SetViewTargetwithBlend (Game|GetPlayerController 0) _returnvalue_2 1.0 "VTBlend_Linear" 0.0 false)
      (Timeline|时间轴_0 PlayFromStart
        (:Finished
          (Variables|Default|SetLeverState 2)
          (Utilities|FlowControl|Delay 1.0)
          (bind _asbp_first_person_character_2 (Utilities|Casting|CastToBP_FirstPersonCharacter (Game|GetPlayerCharacter 0)))
          (Game|Player|SetViewTargetwithBlend (Game|GetPlayerController 0) _asbp_first_person_character_2 1.0 "VTBlend_Linear" 0.0 false))))))

(event EventStopInteract
  ;[0.15 0.15 0.15 0.5] camera & state
  (Pawn|Components|CharacterMovement|SetMovementMode (Variables|/Script/Engine.Character|GetCharacterMovement (stale EventMousePressed _asbp_first_person_character)) "MOVE_Walking" 0)
  (Input|SetIgnoreLookInput (Game|GetPlayerController 0) false)
  (bind _returnvalue (Actor|GetActorOfClass "/Game/Blueprints/BP_lightt.BP_lightt_C"))
  (if (Variables|/Game/Blueprints/BP_lightt.BP_lightt_C|GetState _returnvalue)
    (Variables|Default|SetisHolding false)
    (Utilities|FlowControl|Sequence
      (:then_0
        (Timeline|时间轴_0 Stop
          (:Finished
            (Variables|Default|SetLeverState 2)
            (Utilities|FlowControl|Delay 1.0)
            (bind _asbp_first_person_character (Utilities|Casting|CastToBP_FirstPersonCharacter (Game|GetPlayerCharacter 0)))
            (Game|Player|SetViewTargetwithBlend (Game|GetPlayerController 0) _asbp_first_person_character 1.0 "VTBlend_Linear" 0.0 false))))
      (:then_1
        (bind _asbp_first_person_character_2 (Utilities|Casting|CastToBP_FirstPersonCharacter (Game|GetPlayerCharacter 0)))
        (Game|Player|SetViewTargetwithBlend (Game|GetPlayerController 0) _asbp_first_person_character_2 1.0 "VTBlend_Linear" 0.0 false)))))

(event Input|MouseEvents|LeftMouseButton
  (params (Key :type Key%20Structure :default "None")))

(fn ConstructionScript)

(fn ResetPlayerLogic
  (bind _returnvalue (Game|GetPlayerController 0))
  (Input|SetIgnoreMoveInput _returnvalue false)
  (Input|SetIgnoreLookInput _returnvalue false)
  (bind _asbp_first_person_character (Utilities|Casting|CastToBP_FirstPersonCharacter (Game|GetPlayerCharacter 0)))
  (Pawn|Components|CharacterMovement|SetMovementMode (Variables|/Script/Engine.Character|GetCharacterMovement _asbp_first_person_character) "MOVE_Walking" 0)
  (Game|Player|SetViewTargetwithBlend (Game|GetPlayerController 0) (Game|GetPlayerCharacter 0) 0.0 "VTBlend_Linear" 0.0 false))