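; Interactable elevator button that calls CloseDoor on its referenced door once access is granted and no roots are on it.
; It starts locked with the red indicator lit, and ButtonAccessFunction makes it interactable and switches the lit indicator to green.
; RemoveRootsBool clears the roots flag that blocks Interact.
; Focus events toggle an outline overlay material on the button mesh, which is applied only while it is interactable.
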(event EventBeginPlay
  (Rendering|Material|SetMaterial (Variables|Default|GetButtonGreen) 0 "/Game/LevelPrototyping/Materials/M_FlatCol.M_FlatCol")
  (Rendering|Material|SetMaterial (Variables|Default|GetButtonRed) 0 "/Game/LevelPrototyping/Materials/M_ButtonRed.M_ButtonRed")
  (Variables|Default|SetisInteractable false))

(event Collision|EventActorBeginOverlap
  (params (OtherActor :type Actor%20Object%20Reference))
  (|CallParentFunction OtherActor) ; This node is disabled and will not be called.\nDrag off pins to build functionality.
)

(event EventTick
  (params (DeltaSeconds :type Float%20%28single-precision%29))
  (|CallParentFunction DeltaSeconds) ; This node is disabled and will not be called.\nDrag off pins to build functionality.
)

(event EventRemoveRootsBool
  (Variables|Default|SetHasRootsON false))

(event EventOnFocus
  (if (Variables|Default|GetisInteractable)
    (Rendering|Material|SetOverlayMaterial (Variables|Default|GetButtonMesh) "/Game/LevelPrototyping/Materials/M_InteractOutline.M_InteractOutline" :!class /Script/Engine.MeshComponent)))

(event EventNotonFocus
  (Rendering|Material|SetOverlayMaterial (Variables|Default|GetButtonMesh) 0 :!class /Script/Engine.MeshComponent))

(event EventInteract
  (if (Variables|Default|GetisInteractable)
    (if (not (Variables|Default|GetHasRootsON))
      (Default|CloseDoor (Variables|Default|GetDoorReference)))))

(fn ConstructionScript
  (|CallParentFunction))

(fn ButtonAccessFunction
  (Variables|Default|SetisInteractable true)
  (Rendering|Material|SetMaterial (Variables|Default|GetButtonGreen) 0 "/Game/LevelPrototyping/Materials/M_ButtonGreen.M_ButtonGreen")
  (Rendering|Material|SetMaterial (Variables|Default|GetButtonRed) 0 "/Game/LevelPrototyping/Materials/M_FlatCol.M_FlatCol"))