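; Monster enemy that teleports along a path toward a kill, ending in a jumpscare and Game Over screen.
; Timer ticks advance it by aggression-weighted chance while unwatched; at the path's end, a cancellable kill timer starts, shortened by aggression.
; Being looked at resets it with brief breathing room, raising bloodlust and per-floor capped aggression.
; Bloodlust milestones shorten the path, trigger flickering and finally enable DeathMode, where it advances even while watched.
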(event TimerFinished(Timer)
  ;[0.15 0.15 0.15 0.5] Movement Opertunity
  (if (Variables|Default|GetDeathMode)
    (if (> (Variables|Default|GetBreathingRoom) 0) :!label _label
      (Variables|Default|SetBreathingRoom (- (Variables|Default|GetBreathingRoom) 1))
      (elif (!= (Variables|Default|GetCurrentPosition) (Utilities|Array|LastIndex (Variables|Default|GetPath)))
        (if (< (Math|Random|RandomFloatinRange 0.0 2e+01) (Variables|Default|GetAgression))
          (Variables|Default|SetCurrentPosition (+ (Variables|Default|GetCurrentPosition) 1))
          (Development|PrintString "\"Monster Shift\"")
          (CallFunction|UpdatePosition)
          (CallFunction|MovementSound))
        (else
          ;[0.15 0.15 0.15 0.5] Kill Player
          (if (not (Variables|Default|GetAttemptingKill))
            (Variables|Default|SetAttemptingKill true)
            (bind _returnvalue (Utilities|Time|SetTimerbyEvent (delegate Custom|KillSuccess_Event) (- (Variables|Default|GetKillTimer) (Variables|Default|GetAgression))))))))
    (elif (not (Variables|Default|GetPlayerWatching))
      (goto _label))))

(event Custom|MovementSound
  (bind _returnvalue (Math|Random|RandomIntegerinRange 1 10))
  (bind _creaturebody (Variables|Default|GetCreatureBody))
  (bind _returnvalue_2 (Transformation|GetWorldLocation _creaturebody))
  (if (== _returnvalue 1)
    (Audio|PlaySoundatLocation "/Game/Audio/MonsterSounds/Monster_Claws1.Monster_Claws1" _returnvalue_2 "0, 0, 0" 1.0 1.0 0.0 0 0 0 0)
    (elif (== _returnvalue 2)
      (Audio|PlaySoundatLocation "/Game/Audio/MonsterSounds/Monster_Voices_breaths3.Monster_Voices_breaths3" _returnvalue_2 "0, 0, 0" 1.0 1.0 0.0 0 0 0 0)
      (elif (== _returnvalue 3)
        (Audio|PlaySoundatLocation "/Game/Audio/MonsterSounds/Monster_Claws2.Monster_Claws2" _returnvalue_2 "0, 0, 0" 1.0 1.0 0.0 0 0 0 0)
        (elif (== _returnvalue 4)
          (Audio|PlaySoundatLocation "/Game/Audio/MonsterSounds/Monster_Voices_breaths4.Monster_Voices_breaths4" _returnvalue_2 "0, 0, 0" 1.0 1.0 0.0 0 0 0 0)
          (elif (== _returnvalue 5)
            (Audio|PlaySoundatLocation "/Game/Audio/MonsterSounds/Monster_Voices_breaths5.Monster_Voices_breaths5" _returnvalue_2 "0, 0, 0" 1.0 1.0 0.0 0 0 0 0)
            (elif (== _returnvalue 6)
              (Audio|PlaySoundatLocation "/Game/Audio/MonsterSounds/Monster_Voices_breaths6.Monster_Voices_breaths6" _returnvalue_2 "0, 0, 0" 1.0 1.0 0.0 0 0 0 0))))))))

(event Custom|KillSuccess_Event
  (bind _returnvalue (Game|GetPlayerController 0))
  ;[0.15 0.15 0.15 0.5] Kill Player
  (Development|PrintString "succeeded kill")
  (Default|CallKillPlayer)
  (Development|PrintString "PlayerIsKilled")
  ;[0.15 0.15 0.15 0.5] Jumpscare before game ends
  (bind _asbp_first_person_character (Utilities|Casting|CastToBP_FirstPersonCharacter (Game|GetPlayerCharacter 0)))
  (Default|StartJumpScare _asbp_first_person_character)
  (Audio|PlaySoundatLocation "/Game/Audio/MonsterSounds/Big_Squelch_Kill_Sound.Big_Squelch_Kill_Sound" "0, 0, 0" "0, 0, 0" 1.0 1.0 0.0 0 0 0 0)
  (Utilities|FlowControl|Delay 2.8)
  (Default|EndJumpScare _asbp_first_person_character)
  ;[0.03805 0.000507 0.15 0.5] Monster Kill UI
  (bind _returnvalue_2 (UserInterface|CreateWidget "/Game/UI/Test/WB_GameOver.WB_GameOver_C"))
  (UserInterface|Viewport|AddtoViewport _returnvalue_2 0)
  (Class|Widget|SetCursor _returnvalue_2 "Default")
  (Variables|/Script/Engine.PlayerController|SetbShowMouseCursor _returnvalue true)
  (Input|SetInputModeUIOnly _returnvalue 0 "DoNotLock" false))

(event Custom|PlayerNotLooking
  ;[0.15 0.15 0.15 0.5] FlashedAway
  (Variables|Default|SetPlayerWatching false))

(event Custom|Playerlooking
  (bind _creaturebody (Variables|Default|GetCreatureBody))
  (bind _returnvalue (Transformation|GetWorldLocation _creaturebody))
  ;[0.15 0.15 0.15 0.5] FlashedAway
  (Variables|Default|SetPlayerWatching true)
  (if (!= (Variables|Default|GetCurrentPosition) 0)
    (Utilities|FlowControl|Delay 0.4)
    (Variables|Default|SetCurrentPosition 0)
    (CallFunction|UpdatePosition)
    (Variables|Default|SetBloodlust (+ (Variables|Default|GetBloodlust) 1))
    (CallFunction|CalculateAggression)
    (Variables|Default|SetAttemptingKill false)
    (Variables|Default|SetBreathingRoom 2)
    (CallFunction|PreventKill)
    (CallFunction|BloodlustEvent)
    (if (Math|Random|RandomBool)
      (Audio|PlaySoundatLocation "/Game/Audio/MonsterSounds/Creature_Shrieks.Creature_Shrieks" _returnvalue "0, 0, 0" 1.0 1.0 0.0 0 0 0 0)
      (else
        (Audio|PlaySoundatLocation "/Game/Audio/MonsterSounds/Creature_Shrieks2.Creature_Shrieks2" _returnvalue "0, 0, 0" 1.0 1.0 0.0 0 0 0 0)))))

(event Custom|PreventKill
  ;[0.15 0.15 0.15 0.5] Kill Player
  (Utilities|Time|ClearandInvalidateTimerbyHandle (stale TimerFinished(Timer) _returnvalue)))

(event EventBeginPlay
  ;[0.15 0.15 0.15 0.5] Start()
  (CallFunction|LoadLevel)
  (Input|EnableInput 0)
  (Input|EnableInput (Game|GetPlayerController 0)))

(event Collision|EventActorBeginOverlap
  (params (OtherActor :type Actor%20Object%20Reference)))

(event EventTick
  (params (DeltaSeconds :type Float%20%28single-precision%29)))

(fn ConstructionScript)

(fn UpdatePosition
  (Transformation|SetWorldTransform (Variables|Default|GetCreatureBody) (Math|Conversions|ToTransform(Vector) (Utilities|Array|Get(acopy) (Variables|Default|GetPath) (Variables|Default|GetCurrentPosition))) false true))

(fn CalculateAggression
  (bind _maxagression (Variables|Default|GetMaxAgression))
  (bind _currentfloor (Variables|Default|GetCurrentFloor))
  (bind _output (Utilities|Array|Get(acopy) _maxagression _currentfloor))
  (Variables|Default|SetAgression (+ (Utilities|Array|Get(acopy) (Variables|Default|GetStartingAggression) _currentfloor) (/ (Variables|Default|GetBloodlust) 3)))
  (if (>= (Variables|Default|GetAgression) _output)
    (Variables|Default|SetAgression (Math|Conversions|ToFloat(Integer) _output)))
  (Development|PrintString "*Monster GRRRRR*"))

(fn LoadLevel
  (Variables|Default|SetCurrentFloor (Variables|Default|GetCurrentFloor))
  (Variables|Default|SetAgression (Math|Conversions|ToFloat(Integer) (Utilities|Array|Get(acopy) (Variables|Default|GetStartingAggression) (Variables|Default|GetCurrentFloor))))
  (Variables|Default|SetCurrentPosition 0)
  (CallFunction|UpdatePosition)
  (Variables|Default|SetBloodlust 0)
  (Variables|Default|SetPath (Variables|Default|GetPositons))
  (Variables|Default|SetAttemptingKill false)
  (Variables|Default|SetDeathMode false))

(fn BloodlustEvent
  (bind _bloodlust (Variables|Default|GetBloodlust))
  (if (!= _bloodlust 3)
    (if (!= _bloodlust 6)
      (if (!= _bloodlust 9)
        (if (not (!= _bloodlust 12))
          (Development|PrintString "Bloodlust Event 4 Active")
          (Variables|Default|SetDeathMode true)
          (Audio|PlaySoundatLocation "/Game/Audio/MonsterSounds/monster_anger4.monster_anger4" (Transformation|GetWorldLocation (Variables|Default|GetCreatureBody)) "0, 0, 0" 1.0 1.0 0.0 0 0 0 0))
        (else
          (Development|PrintString "Bloodlust Event 3 Active")
          (Utilities|Array|RemoveIndex (Variables|Default|GetPath) 2)
          (Audio|PlaySoundatLocation "/Game/Audio/MonsterSounds/monster_anger3.monster_anger3" (Transformation|GetWorldLocation (Variables|Default|GetCreatureBody)) "0, 0, 0" 1.0 1.0 0.0 0 0 0 0)))
      (else
        (Development|PrintString "Bloodlust Event 2 Active")
        (bind _returnvalue (Actor|GetActorOfClass "/Game/FirstPerson/Blueprints/BP_FirstPersonCharacter.BP_FirstPersonCharacter_C"))
        (Default|StartFlickering _returnvalue)
        (Audio|PlaySoundatLocation "/Game/Audio/MonsterSounds/monster_anger2.monster_anger2" (Transformation|GetWorldLocation (Variables|Default|GetCreatureBody)) "0, 0, 0" 1.0 1.0 0.0 0 0 0 0)))
    (else
      (Development|PrintString "Bloodlust Event 1 Active")
      (Utilities|Array|RemoveIndex (Variables|Default|GetPath) 1)
      (Audio|PlaySoundatLocation "/Game/Audio/MonsterSounds/monster_anger1.monster_anger1" (Transformation|GetWorldLocation (Variables|Default|GetCreatureBody)) "0, 0, 0" 1.0 1.0 0.0 0 0 0 0))))

(fn NewFunction)