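; Temporary holding Blueprint for monster sound logic, with almost all of its nodes unconnected.
; The MovementSound event walks a chain of random rolls, rerolled at each branch, to play one claw or breath sound at CreatureBody, or none.
; Unwired fragments hold further breath variants, flashed-away shrieks, a bloodlust anger sound, first-person pipe grab/drop scrapes, the MovementSound trigger and an unused audio component array.
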(event Custom|MovementSound
  (bind _returnvalue (Math|Random|RandomIntegerinRange 1 10))
  (bind _creaturebody (Variables|Default|GetCreatureBody))
  (bind _returnvalue_2 (Transformation|GetWorldLocation _creaturebody))
  ;[0.15 0.15 0.15 0.5] MovementSound Random
  (if (== _returnvalue 1)
    (Audio|PlaySoundatLocation "/Game/Audio/MonsterSounds/Monster_Claws1.Monster_Claws1" _returnvalue_2 "0, 0, 0" 1.0 1.0 0.0 0 0 0 0)
    (elif (== _returnvalue 2)
      (Audio|PlaySoundatLocation "/Game/Audio/MonsterSounds/Monster_Voices_breaths3.Monster_Voices_breaths3" _returnvalue_2 "0, 0, 0" 1.0 1.0 0.0 0 0 0 0)
      (elif (== _returnvalue 3)
        (Audio|PlaySoundatLocation "/Game/Audio/MonsterSounds/Monster_Claws2.Monster_Claws2" _returnvalue_2 "0, 0, 0" 1.0 1.0 0.0 0 0 0 0)
        (elif (== _returnvalue 4)
          (Audio|PlaySoundatLocation "/Game/Audio/MonsterSounds/Monster_Voices_breaths4.Monster_Voices_breaths4" _returnvalue_2 "0, 0, 0" 1.0 1.0 0.0 0 0 0 0)
          (elif (== _returnvalue 5)
            (Audio|PlaySoundatLocation "/Game/Audio/MonsterSounds/Monster_Voices_breaths5.Monster_Voices_breaths5" _returnvalue_2 "0, 0, 0" 1.0 1.0 0.0 0 0 0 0)
            (elif (== _returnvalue 6)
              (Audio|PlaySoundatLocation "/Game/Audio/MonsterSounds/Monster_Voices_breaths6.Monster_Voices_breaths6" _returnvalue_2 "0, 0, 0" 1.0 1.0 0.0 0 0 0 0))))))))

(event EventBeginPlay)

(event Collision|EventActorBeginOverlap
  (params (OtherActor :type Actor%20Object%20Reference)))

(event EventTick
  (params (DeltaSeconds :type Float%20%28single-precision%29)))

(fn ConstructionScript)