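; BP_LSElevator is an elevator actor that gives its static mesh a swaying motion, with no travel logic in this graph.
; On BeginPlay it stores the mesh's world location and plays the ElevatorSway timeline.
; Each update offsets that stored location along the mesh's right and up vectors by the Sway track, more strongly sideways than vertically.
; The result is applied as a relative location, although the stored base is in world space.
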(event Collision|EventActorBeginOverlap
  (params (OtherActor :type Actor%20Object%20Reference)))

(event EventTick
  (params (DeltaSeconds :type Float%20%28single-precision%29)))

(event EventBeginPlay
  (Variables|Default|SetbaseLocation (Transformation|GetWorldLocation (Variables|Debug|GetStaticMeshComponent)))
  (bind _sway (Timeline|ElevatorSway Play)
    (:Update
      (Transformation|SetRelativeLocation (Variables|Debug|GetStaticMeshComponent) (+ (Variables|Default|GetbaseLocation) (* (Math|Vector|GetRightVector (Variables|Debug|GetStaticMeshComponent)) _sway "1.500000,1.500000,1.500000") (* (Math|Vector|GetUpVector (Variables|Debug|GetStaticMeshComponent)) _sway "0.600000,0.600000,0.600000")) false false))))

(fn ConstructionScript)