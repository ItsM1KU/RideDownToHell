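; Task manager actor that tracks how many level tasks are done and reacts when all are completed.
; On BeginPlay it sets the required total to the number of actors implementing BPI_Tasks.
; CheckIfTasksComplete recounts solved tasks through that interface and calls CloseDoor on the referenced elevator door when all are solved.
; Separately, TaskComplete increments the same counter and, once only, prints a message and calls AllTasksCompleted.
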(event Custom|CheckIfTasksComplete
  (Variables|Default|SetCompletedTasks 0)
  (bind _outactors (Actor|GetAllActorswithInterface "/Game/Blueprints/BPI_Tasks.BPI_Tasks_C"))
  (for _array_element _outactors
    (bind _issolved (Class|BPITasks|CheckIsSolved(Message) _array_element))
    (if _issolved
      (bind _result (Math|Integer|IncrementInt (Variables|Default|GetCompletedTasks))
        (:%20%20
          (Variables|Default|SetCompletedTasks _result)
          (if (== (Variables|Default|GetCompletedTasks) (Variables|Default|GetRequiredTasks))
            (Default|CloseDoor (Variables|Default|GetElevatorDoorReference))))))))

(event EventBeginPlay
  (Variables|Default|SetCompletedTasks 0)
  (bind _outactors (Actor|GetAllActorswithInterface "/Game/Blueprints/BPI_Tasks.BPI_Tasks_C"))
  (Variables|Default|SetRequiredTasks (Utilities|Array|Length _outactors))
  (Variables|Default|SetbAlreadyCompleted false))

(event Collision|EventActorBeginOverlap
  (params (OtherActor :type Actor%20Object%20Reference)))

(event EventTick
  (params (DeltaSeconds :type Float%20%28single-precision%29)))

(fn ConstructionScript)

(fn TaskComplete
  (if (not (Variables|Default|GetbAlreadyCompleted))
    (bind _result (Math|Integer|IncrementInt (Variables|Default|GetCompletedTasks))
      (:%20%20
        (Variables|Default|SetCompletedTasks _result)
        (if (>= (Variables|Default|GetCompletedTasks) (Variables|Default|GetRequiredTasks))
          (Development|PrintString "All tasks Completed!!")
          (Variables|Default|SetbAlreadyCompleted true)
          (Default|CallAllTasksCompleted))))))