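; BP_ControlPanel is an interactable computer that opens a control panel puzzle widget as one of the player's tasks.
; It creates the widget at BeginPlay, and interacting displays it with UI-only input and player movement disabled.
; Closing restores controls and, if the widget is complete, marks the panel complete and has the character's TaskManager check all tasks.
; Focus outlines the computer via an overlay material while it is interactable and incomplete.
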(event Custom|ClosePaneUI
  (bind _controlpanelui (Variables|Default|GetControlPanelUI))
  (Utilities|IsValid _controlpanelui
    (:Is%20Valid
      (Widget|RemovefromParent _controlpanelui)
      (Class|Widget|SetCursor _controlpanelui "None")
      (Input|SetInputModeGameOnly (Game|GetPlayerController 0) false)
      (Pawn|Components|CharacterMovement|SetMovementMode (Variables|/Script/Engine.Character|GetCharacterMovement (Game|GetPlayerCharacter 0)) "MOVE_Walking" 0)
      (if (Variables|/Game/UI/Test/WBP_ControlPanel.WBP_ControlPanel_C|GetisComplete (Variables|Default|GetControlPanelUI))
        (Variables|Default|SetisComplete true)
        (bind _asbp_first_person_character (Utilities|Casting|CastToBP_FirstPersonCharacter (Game|GetPlayerCharacter 0)))
        (Default|CheckifTasksComplete (Variables|/Game/FirstPerson/Blueprints/BP_FirstPersonCharacter.BP_FirstPersonCharacter_C|GetTaskManagerRef _asbp_first_person_character))))))

(event EventInteract
  (bind _controlpanelui (Variables|Default|GetControlPanelUI))
  (if (Variables|Default|GetisInteractable)
    (UserInterface|Viewport|AddtoViewport _controlpanelui 0)
    (Class|Widget|SetCursor _controlpanelui "Default")
    (Input|SetInputModeUIOnly (Game|GetPlayerController 0) (Variables|Default|GetControlPanelUI) "DoNotLock" false)
    (Pawn|Components|CharacterMovement|SetMovementMode (Variables|/Script/Engine.Character|GetCharacterMovement (Game|GetPlayerCharacter 0)) "MOVE_None" 0)))

(event EventOnFocus
  ;[0.15 0.15 0.15 0.5] UI
  (if (Variables|Default|GetisInteractable)
    (if (not (Variables|Default|GetisComplete))
      (Rendering|Material|SetOverlayMaterial (Variables|Default|GetComputer) "/Game/LevelPrototyping/Materials/M_InteractOutline.M_InteractOutline" :!class /Script/Engine.MeshComponent))))

(event EventNotonFocus
  ;[0.15 0.15 0.15 0.5] UI
  (Rendering|Material|SetOverlayMaterial (Variables|Default|GetComputer) 0 :!class /Script/Engine.MeshComponent))

(event EventBeginPlay
  (bind _returnvalue (UserInterface|CreateWidget "/Game/UI/Test/WBP_ControlPanel.WBP_ControlPanel_C"))
  (Variables|Default|SetControlPanelUI _returnvalue)
  (Variables|/Game/UI/Test/WBP_ControlPanel.WBP_ControlPanel_C|SetControlPanelRef _returnvalue self)
  (Variables|Default|SetisComplete false))

(fn ConstructionScript
  (|CallParentFunction))

(fn CheckifIsComplete
  (bind _controlpanelui (Variables|Default|GetControlPanelUI))
  (Default|CheckAllBarsComplete _controlpanelui)
  (if (Variables|/Game/UI/Test/WBP_ControlPanel.WBP_ControlPanel_C|GetisComplete _controlpanelui)
    (Variables|Default|SetisComplete true))
  (return (Variables|/Game/UI/Test/WBP_ControlPanel.WBP_ControlPanel_C|GetisComplete _controlpanelui)))