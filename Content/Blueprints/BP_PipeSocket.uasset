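; BP_PipeSocket is a task socket that holds one pipe, starting with any assigned InsertedPart snapped into it.
; Box overlaps register a "ChangeablePipe"-tagged actor as compatible while empty and clear the inserted pipe when it leaves.
; TryInsert snaps the compatible pipe in, disables its physics and collision, marks completion and updates the player's TaskManager.
; Query functions expose interactable state, solved state and task type.
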(event OnComponentEndOverlap(Box)
  (params (OverlappedComponent :type Primitive%20Component%20Object%20Reference) (OtherActor :type Actor%20Object%20Reference) (OtherComp :type Primitive%20Component%20Object%20Reference) (OtherBodyIndex :type Integer))
  (Utilities|IsValid (Variables|Default|GetinsertedPart)
    (:Is%20Valid
      (if (== (Variables|Default|GetinsertedPart) OtherActor)
        (Variables|Default|SetinsertedPart 0)
        (Development|PrintString "Inserted Part is removed!!")
        (Development|PrintString "Old Pipe removed so stop the steam")
        (elif (== OtherActor (Variables|Default|GetcompatiblePart))
          (Variables|Default|SetcompatiblePart 0)
          (Development|PrintString "Compatible Part is removed!!"))))))

(event OnComponentBeginOverlap(Box)
  (params (OverlappedComponent :type Primitive%20Component%20Object%20Reference) (OtherActor :type Actor%20Object%20Reference) (OtherComp :type Primitive%20Component%20Object%20Reference) (OtherBodyIndex :type Integer) (bFromSweep :type Boolean) (SweepResult :type Hit%20Result%20Structure%20%28by%20ref%29))
  (Utilities|IsValid (Variables|Default|GetinsertedPart)
    (:Is%20Valid
      (Development|PrintString "There is already a pipe here!!"))
    (:Is%20Not%20Valid
      (if (Actor|ActorHasTag OtherActor "ChangeablePipe")
        (Variables|Default|SetcompatiblePart OtherActor)
        (Development|PrintString "New pipe has become compatible")))))

(event EventBeginPlay
  (Transformation|SetActorLocation (Variables|Default|GetinsertedPart) (Transformation|GetActorLocation) false false))

(fn ConstructionScript)

(fn TryInsert
  (params (PipeActor :type Actor%20Object%20Reference))
  (Utilities|IsValid (Variables|Default|GetinsertedPart)
    (:Is%20Not%20Valid
      (Utilities|IsValid (Variables|Default|GetcompatiblePart)
        (:Is%20Valid
          (if (== PipeActor (Variables|Default|GetcompatiblePart))
            (Variables|Default|SetinsertedPart (Variables|Default|GetcompatiblePart))
            (Variables|Default|SetcompatiblePart 0)
            (Transformation|SetActorLocationAndRotation (Variables|Default|GetinsertedPart) (Transformation|GetWorldLocation (Variables|Default|GetDefaultSceneRoot)))
            (Physics|SetSimulatePhysics (Actor|GetComponentbyClass (Variables|Default|GetinsertedPart) "/Script/Engine.StaticMeshComponent") false)
            (Collision|SetCollisionEnabled (Actor|GetComponentbyClass (Variables|Default|GetinsertedPart) "/Script/Engine.StaticMeshComponent") "NoCollision")
            (Variables|Default|SetisComplete true)
            (bind _asbp_first_person_character (Utilities|Casting|CastToBP_FirstPersonCharacter (Game|GetPlayerCharacter 0)))
            (Default|UpdateTaskData (Variables|/Game/FirstPerson/Blueprints/BP_FirstPersonCharacter.BP_FirstPersonCharacter_C|GetTaskManagerRef _asbp_first_person_character))))))))

(fn CheckIsInteractable
  (return (Variables|Default|GetisInteractable)))

(fn CheckIsSolved
  (return (Variables|Default|GetisComplete)))

(fn TaskType
  (return "NewEnumerator2"))