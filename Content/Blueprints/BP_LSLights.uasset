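; BP_LSLights is an actor that lights six light balls one at a time through their materials' GlowFactor parameter.
; BeginPlay gathers Light1 to Light6 into an array, switches each off and calls Play on the LightGlowLoop timeline inside that same loop.
; On each timeline update, the floored LightValue selects the array index that glows, and every other ball is set dark.
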(event Collision|EventActorBeginOverlap
  (params (OtherActor :type Actor%20Object%20Reference)))

(event EventTick
  (params (DeltaSeconds :type Float%20%28single-precision%29)))

(event EventBeginPlay
  (bind _output_get (Variables|Default|SetlightBalls (Utilities|Array|MakeArray (Variables|Default|GetLight1) (Variables|Default|GetLight2) (Variables|Default|GetLight3) (Variables|Default|GetLight4) (Variables|Default|GetLight5) (Variables|Default|GetLight6))))
  (for _array_element _output_get
    (Rendering|Material|SetScalarParameterValueonMaterials _array_element "GlowFactor" 0.0)
    (bind _lightvalue (Timeline|LightGlowLoop Play)
      (:Update
        (for (_array_element_2 _array_index) (Variables|Default|GetlightBalls)
          (if (== _array_index (Math|Float|Floor _lightvalue))
            (Rendering|Material|SetScalarParameterValueonMaterials _array_element_2 "GlowFactor" 1.0)
            (else
              (Rendering|Material|SetScalarParameterValueonMaterials _array_element_2 "GlowFactor" 0.0))))))))

(fn ConstructionScript)