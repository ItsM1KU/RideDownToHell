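; Wire-matching puzzle actor: clicking can swing its door open once, which enables Tick so cables can be dragged between tagged endpoints.
; While the player's Click is held, Tick traces from the camera for "L" endpoints and attaches the matching cable to the player's Sphere.
; Mouse release snaps it to an "R" endpoint with the same second tag, otherwise to FailPoint.
; Five matches print success and disable Tick.
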(event Collision|EventActorBeginOverlap
  (params (OtherActor :type Actor%20Object%20Reference)))

(event EventTick
  (params (DeltaSeconds :type Float%20%28single-precision%29))
  (Utilities|FlowControl|Sequence
    (:then_1
      (bind _asbp_first_person_character (Utilities|Casting|CastToBP_FirstPersonCharacter (Game|GetPlayerCharacter 0)))
      (if (Variables|/Game/FirstPerson/Blueprints/BP_FirstPersonCharacter.BP_FirstPersonCharacter_C|GetClick _asbp_first_person_character)
        (bind _outhit (Collision|LineTraceByChannel (Transformation|GetWorldLocation (Variables|/Script/RideDownToHell.RideDownToHellCharacter|GetFirstPersonCameraComponent _asbp_first_person_character)) (+ (Transformation|GetWorldLocation (Variables|/Script/RideDownToHell.RideDownToHellCharacter|GetFirstPersonCameraComponent _asbp_first_person_character)) (* (Math|Vector|GetForwardVector (Variables|/Script/RideDownToHell.RideDownToHellCharacter|GetFirstPersonCameraComponent _asbp_first_person_character)) 1000)) "TraceTypeQuery1" false 0 "None"))
        (if (or (Components|ComponentHasTag (.HitComponent (Collision|BreakHitResult _outhit)) "L") (Actor|ActorHasTag (.HitActor (Collision|BreakHitResult _outhit)) "L"))
          (if (< (Math|Vector|Distance(Vector) (Transformation|GetWorldLocation (Variables|Default|GetCable)) (Transformation|GetWorldLocation (Variables|/Game/FirstPerson/Blueprints/BP_FirstPersonCharacter.BP_FirstPersonCharacter_C|GetSphere _asbp_first_person_character))) 9e+01)
            (bind _output_get (Variables|Default|SetCurrentCable (Utilities|Array|Get(acopy) (Actor|GetComponentsbyTag "/Script/CableComponent.CableComponent" (Utilities|Array|Get(acopy) (Variables|/Script/Engine.ActorComponent|GetComponentTags (.HitComponent (Collision|BreakHitResult _outhit))) 1)))))
            (Class|CableComponent|SetAttachEndtoComponent _output_get (Variables|/Game/FirstPerson/Blueprints/BP_FirstPersonCharacter.BP_FirstPersonCharacter_C|GetSphere _asbp_first_person_character) "None")
            (Variables|Default|SetSourceNumber (Utilities|Array|Get(acopy) (Variables|/Script/Engine.ActorComponent|GetComponentTags (.HitComponent (Collision|BreakHitResult _outhit))) 1))
            (Variables|Default|SetCurrentBall (.HitComponent (Collision|BreakHitResult _outhit)))))))))

(event EventBeginPlay
  (Actor|Tick|SetActorTickEnabled false))

(event EventMouseReleased
  (bind _asbp_first_person_character (Utilities|Casting|CastToBP_FirstPersonCharacter (Game|GetPlayerCharacter 0)))
  (bind _outhit (Collision|LineTraceByChannel (Transformation|GetWorldLocation (Variables|/Script/RideDownToHell.RideDownToHellCharacter|GetFirstPersonCameraComponent _asbp_first_person_character)) (+ (Transformation|GetWorldLocation (Variables|/Script/RideDownToHell.RideDownToHellCharacter|GetFirstPersonCameraComponent _asbp_first_person_character)) (* (Math|Vector|GetForwardVector (Variables|/Script/RideDownToHell.RideDownToHellCharacter|GetFirstPersonCameraComponent _asbp_first_person_character)) 1000)) "TraceTypeQuery1" false 0 "None"))
  (if (== (Utilities|Array|Get(acopy) (Variables|/Script/Engine.ActorComponent|GetComponentTags (.HitComponent (Collision|BreakHitResult _outhit)))) "R")
    (if (== (Utilities|Array|Get(acopy) (Variables|/Script/Engine.ActorComponent|GetComponentTags (.HitComponent (Collision|BreakHitResult _outhit))) 1) (Variables|Default|GetSourceNumber))
      (Class|CableComponent|SetAttachEndtoComponent (Variables|Default|GetCurrentCable) (.HitComponent (Collision|BreakHitResult _outhit)) "None")
      (Variables|Default|SetCurrentCable 0)
      (Collision|SetCollisionEnabled (Variables|Default|GetCurrentBall) "NoCollision")
      (Variables|Default|SetCurrentBall 0)
      (bind _output_get (Variables|Default|SetFixedWires (+ (Variables|Default|GetFixedWires) 1)))
      (if (== _output_get 5)
        (Development|PrintString "success")
        (Actor|Tick|SetActorTickEnabled false))
      (else
        (Utilities|IsValid (Variables|Default|GetCurrentCable) :!label _label
          (:Is%20Valid
            (Class|CableComponent|SetAttachEndtoComponent (Variables|Default|GetCurrentCable) (Variables|Default|GetFailPoint) "None")))))
    (else
      (goto _label))))

(event EventMousePressed
  (bind _asbp_first_person_character (Utilities|Casting|CastToBP_FirstPersonCharacter (Game|GetPlayerCharacter 0)))
  (if (< (Math|Vector|Distance(Vector) (Transformation|GetWorldLocation (Variables|/Script/Engine.Actor|GetRootComponent _asbp_first_person_character)) (Transformation|GetWorldLocation (Variables|/Game/FirstPerson/Blueprints/BP_FirstPersonCharacter.BP_FirstPersonCharacter_C|GetSphere _asbp_first_person_character))) 9e+01)
    (Utilities|FlowControl|DoOnce false
      (:Completed
        (bind _新建轨道_0 (Timeline|时间轴 Play)
          (:Update
            (Transformation|SetRelativeRotation (Variables|Default|Getdoor) (Math|Rotator|MakeRotator 0.0 0.0 (Math|Float|Lerp 0.0 -1.2e+02 _新建轨道_0)) false false)
            (Actor|Tick|SetActorTickEnabled true)))))))

(fn ConstructionScript)