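; BP_Elevator is a one-shot elevator that moves a platform to an end point and then opens two doors.
; ActivateElevator, guarded by an Activated flag, uses a timeline to lerp the platform's world location to EndPoint.
; After a configurable delay, OpenDoors runs a second timeline offsetting each door's relative location.
; The left door moves along Z with an extra multiplier, while the right moves along X.
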(event Custom|ActivateElevator
  (Development|PrintString "ActivateElevator")
  (if (not (Variables|Default|GetbActivated))
    (Variables|Default|SetbActivated true)
    (Variables|Default|SetPlatformStartLoc (Transformation|GetWorldLocation (Variables|组件|GetPlatform)))
    (Variables|Default|SetPlatformEndLoc (Transformation|GetWorldLocation (Variables|组件|GetEndPoint)))
    (bind _alpha (Timeline|TL_MovePlatform PlayFromStart)
      (:Update
        (Transformation|SetWorldLocation (Variables|组件|GetPlatform) (Math|Vector|Lerp(Vector) (Variables|Default|GetPlatformStartLoc) (Variables|Default|GetPlatformEndLoc) _alpha) false false))
      (:Finished
        (Development|PrintString "Platform Finished")
        (Utilities|FlowControl|Delay (Variables|Default|GetWaitBeforeOpen))
        (CallFunction|OpenDoors)))))

(event Custom|OpenDoors
  (Development|PrintString "opendoors")
  (Variables|Default|SetDoorLeftStartLoc (Variables|/Script/Engine.SceneComponent|GetRelativeLocation (Variables|组件|GetDoorLeft)))
  (Variables|Default|SetDoorRightStartLoc (Variables|/Script/Engine.SceneComponent|GetRelativeLocation (Variables|组件|GetDoorRight)))
  (bind _alpha (Timeline|TL_OpenDoors PlayFromStart)
    (:Update
      (Transformation|SetRelativeLocation (Variables|组件|GetDoorLeft) (+ (Variables|Default|GetDoorLeftStartLoc) (Math|Vector|MakeVector 0.0 0.0 (* (* _alpha (Variables|Default|GetDoorOpenDistance)) 8e+01))) false false)
      (Transformation|SetRelativeLocation (Variables|组件|GetDoorRight) (+ (Variables|Default|GetDoorRightStartLoc) (Math|Vector|MakeVector (* _alpha (Variables|Default|GetDoorOpenDistance)) 0.0 0.0)) false false))))

(event EventBeginPlay)

(event Collision|EventActorBeginOverlap
  (params (OtherActor :type Actor%20Object%20Reference)))

(event EventTick
  (params (DeltaSeconds :type Float%20%28single-precision%29)))

(fn ConstructionScript)