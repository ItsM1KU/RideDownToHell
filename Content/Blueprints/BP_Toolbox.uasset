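; Interactable toolbox that dispenses the tool currently selected on its attached WBP_Toolbox widget, which can be disabled.
; Right-click cycles the available tools and refreshes the widget's name and icon.
; Interacting either spawns a replacement pipe once, provided the player holds no knife, or toggles the player's knife, with sounds.
; Focus adds an outline overlay and shows toolbox help through the crosshair widget.
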(event EventOnFocus
  (Rendering|Material|SetOverlayMaterial (Variables|Default|Gettoolbox) "/Game/LevelPrototyping/Materials/M_InteractOutline.M_InteractOutline" :!class /Script/Engine.MeshComponent)
  (bind _foundwidgets (Widget|GetAllWidgetsOfClass "/Game/UI/Images/WBP_Crosshair.WBP_Crosshair_C" true))
  (for _array_element _foundwidgets
    (Default|ToolboxHelp (Variables|/Game/UI/Images/WBP_Crosshair.WBP_Crosshair_C|GetTipREF _array_element))))

(event EventNotonFocus
  (Rendering|Material|SetOverlayMaterial (Variables|Default|Gettoolbox) 0 :!class /Script/Engine.MeshComponent))

(event EventBeginPlay
  (if (Variables|Default|GetUIDisabled?)
    (Rendering|SetVisibility (Variables|Default|GetWidget) false false)
    (else
      (Rendering|SetVisibility (Variables|Default|GetWidget) true false)
      (Variables|Default|SetisPipeSpawned false)
      (bind _aswbp_toolbox (Utilities|Casting|CastToWBP_Toolbox (UserInterface|GetUserWidgetObject (Variables|Default|GetWidget))))
      (Variables|Default|SetToolboxUIRef _aswbp_toolbox)
      (CallFunction|UpdateUI))))

(event EventInteract
  (bind _spawnpoint (Variables|Default|GetSpawnPoint))
  (bind _defaultsceneroot (Variables|Default|GetDefaultSceneRoot))
  (bind _returnvalue (Transformation|GetWorldLocation _defaultsceneroot))
  (bind _returnvalue_2 (Transformation|GetWorldLocation _spawnpoint))
  (switch Utilities|FlowControl|Switch|SwitchonE_Tools (Variables|Default|GetSelectedTool)
    (:NewEnumerator1
      (if (not (Variables|Default|GetisPipeSpawned))
        (bind _asbp_first_person_character (Utilities|Casting|CastToBP_FirstPersonCharacter (Game|GetPlayerCharacter 0)))
        (if (not (Variables|/Game/FirstPerson/Blueprints/BP_FirstPersonCharacter.BP_FirstPersonCharacter_C|GetisHoldingKnife _asbp_first_person_character))
          (Variables|Default|SetisPipeSpawned true)
          (Game|SpawnActorfromClass "/Game/Blueprints/BP_changepipe.BP_changepipe_C" (Math|Conversions|ToTransform(Vector) _returnvalue_2) "Undefined" "MultiplyWithRoot" 0 0)
          (Audio|PlaySoundatLocation "/Game/Audio/ActiveSounds/ValveCreaks/Valve_Creaks3.Valve_Creaks3" _returnvalue_2 "0, 0, 0" 1.0 1.0 0.0 0 0 0 0))))
    (:NewEnumerator2
      (bind _asbp_first_person_character_2 (Utilities|Casting|CastToBP_FirstPersonCharacter (Game|GetPlayerCharacter 0)))
      (if (Variables|/Game/FirstPerson/Blueprints/BP_FirstPersonCharacter.BP_FirstPersonCharacter_C|GetisHoldingKnife _asbp_first_person_character_2)
        (Default|UnequipKnife _asbp_first_person_character_2)
        (Audio|PlaySoundatLocation "/Game/Audio/ActiveSounds/Returning_a_Tool.Returning_a_Tool" _returnvalue "0, 0, 0" 1.0 1.0 0.0 0 0 0 0)
        (else
          (Default|EquipKnife _asbp_first_person_character_2)
          (Audio|PlaySoundatLocation "/Game/Audio/ActiveSounds/Taking_a_Tool_out_of_the_box.Taking_a_Tool_out_of_the_box" _returnvalue "0, 0, 0" 1.0 1.0 0.0 0 0 0 0))))))

(event EventMouseRightButton
  (Variables|Default|SetcurrentIndex (Math|Integer|%(Integer) (+ (Variables|Default|GetcurrentIndex) 1) (Utilities|Array|Length (Variables|Default|GetAvailableTools))))
  (Variables|Default|SetSelectedTool (Utilities|Array|Get(acopy) (Variables|Default|GetAvailableTools) (Variables|Default|GetcurrentIndex)))
  (CallFunction|UpdateUI))

(fn ConstructionScript
  (|CallParentFunction))

(fn UpdateUI
  (bind _toolboxuiref (Variables|Default|GetToolboxUIRef))
  (switch Utilities|FlowControl|Switch|SwitchonE_Tools (Variables|Default|GetSelectedTool)
    (:NewEnumerator0
      (Default|UpdateUI _toolboxuiref "None" "/Game/UI/Images/crosshair.crosshair"))
    (:NewEnumerator1
      (Default|UpdateUI _toolboxuiref "Pipe" "/Game/UI/Images/ClickTest.ClickTest"))
    (:NewEnumerator2
      (Default|UpdateUI _toolboxuiref "Knife" "/Game/UI/Images/ClickTest.ClickTest"))))