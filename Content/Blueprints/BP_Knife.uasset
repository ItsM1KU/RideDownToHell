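; BP_Knife is a knife pickup that the first-person player character can interact with to equip a knife.
; Focus events toggle an outline overlay material on the Knife component to highlight it.
; Interacting casts the player character to BP_FirstPersonCharacter, calls its EquipKnife, clears its FocusedActor and destroys the pickup.
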(event EventInteract
  (bind _asbp_first_person_character (Utilities|Casting|CastToBP_FirstPersonCharacter (Game|GetPlayerCharacter 0)))
  (Default|EquipKnife _asbp_first_person_character)
  (Variables|/Game/FirstPerson/Blueprints/BP_FirstPersonCharacter.BP_FirstPersonCharacter_C|SetFocusedActor _asbp_first_person_character 0)
  (Actor|DestroyActor))

(event EventOnFocus
  (Rendering|Material|SetOverlayMaterial (Variables|Default|GetKnife) "/Game/LevelPrototyping/Materials/M_InteractOutline.M_InteractOutline" :!class /Script/Engine.MeshComponent))

(event EventNotonFocus
  (Rendering|Material|SetOverlayMaterial (Variables|Default|GetKnife) 0 :!class /Script/Engine.MeshComponent))

(fn ConstructionScript)