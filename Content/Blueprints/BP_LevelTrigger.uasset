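; Level trigger Blueprint that advances the game to the next level when its TriggerLevelChange event is called.
; It stores the next player spawn transform in BP_GameInstance and increments the current level index there.
; Past the third index it only prints a game-end message; otherwise it shows a WBP_Fade fade-in, waits briefly, then opens the configured next level.
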(event Custom|TriggerLevelChange
  (Development|PrintString "Level Trigger Happened")
  (bind _asbp_game_instance (Utilities|Casting|CastToBP_GameInstance (Game|GetGameInstance)))
  (Variables|/Game/UI/Menu/BP_GameInstance.BP_GameInstance_C|SetPlayerSpawnTransform _asbp_game_instance (Variables|Default|GetNext%20Level%20Player%20Spawn%20Transform))
  (bind _result (Math|Integer|IncrementInt (Variables|/Game/UI/Menu/BP_GameInstance.BP_GameInstance_C|GetCurrentLevelIndex _asbp_game_instance))
    (:%20%20
      (bind _output_get (Variables|/Game/UI/Menu/BP_GameInstance.BP_GameInstance_C|SetCurrentLevelIndex _asbp_game_instance _result))
      (if (> _output_get 3)
        (Development|PrintString "Game End!!")
        (else
          (bind _returnvalue (UserInterface|CreateWidget "/Game/Blueprints/WBP_Fade.WBP_Fade_C"))
          (UserInterface|Viewport|AddtoViewport _returnvalue 0)
          (Default|Fadein _returnvalue)
          (Utilities|FlowControl|Delay 1.0)
          (Game|OpenLevel(byObjectReference) (Variables|Default|GetNextLevelToLoad)))))))

(fn ConstructionScript)