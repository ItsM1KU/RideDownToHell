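; Wire-matching puzzle actor in which the player drags colored cables from left terminals to right terminals of the same color.
; A left click traces under the cursor, identifies the terminal by component tag, and selects its cable and required target tag unless completed.
; Tick moves the cable end to the cursor hit.
; Release either snaps it to a matching terminal and marks that wire completed, or hides it.
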(event OnInputTouchBegin(L_Red)
  (params (FingerIndex :type ETouchIndex%20Enum :default "Touch1") (TouchedComponent :type Primitive%20Component%20Object%20Reference))
  (bind _cable_red (Variables|Default|GetCable_Red))
  (Variables|Default|SetRequired%20Tag "RRED")
  (Variables|Default|SetCurrentCable _cable_red)
  (Rendering|SetVisibility _cable_red true false)
  (Variables|Default|SetIsDragging true))

(event EventBeginPlay
  (bind _returnvalue (Game|GetPlayerController 0))
  (Variables|/Script/Engine.PlayerController|SetbShowMouseCursor _returnvalue true)
  (Variables|/Script/Engine.PlayerController|SetbEnableClickEvents _returnvalue true))

(event Collision|EventActorBeginOverlap
  (params (OtherActor :type Actor%20Object%20Reference)))

(event EventTick
  (params (DeltaSeconds :type Float%20%28single-precision%29))
  (bind _currentcable (Variables|Default|GetCurrentCable))
  (if (Variables|Default|GetIsDragging)
    (Variables|/Script/CableComponent.CableComponent|SetEndLocation _currentcable (Math|Transform|InverseTransformLocation (Transformation|GetWorldTransform _currentcable) (.Location (Collision|BreakHitResult (.HitResult (Game|Player|GetHitResultUnderCursorbyChannel (Game|GetPlayerController 0) "TraceTypeQuery1" true))))))))

(event Input|MouseEvents|LeftMouseButton
  (params (Key :type Key%20Structure :default "None"))
  (bind _returnvalue (Game|GetPlayerController 0))
  (bind _returnvalue_2 (Game|GetPlayerController 0))
  (bind _cable_red (Variables|Default|GetCable_Red))
  (bind _cable_blue (Variables|Default|GetCable_Blue))
  (bind _cable_green (Variables|Default|GetCable_Green))
  (bind _cable_yellow (Variables|Default|GetCable_Yellow))
  (bind _hitresult (Game|Player|GetHitResultUnderCursorbyChannel _returnvalue "TraceTypeQuery1" true))
  (bind _hitresult_2 (Game|Player|GetHitResultUnderCursorbyChannel _returnvalue_2 "TraceTypeQuery1" true))
  (bind _hitcomponent (Collision|BreakHitResult _hitresult))
  (bind (_bblockinghit _binitialoverlap _time _distance _location _impactpoint _normal _impactnormal _physmat _hitactor _hitcomponent_2) (Collision|BreakHitResult _hitresult_2))
  (:Pressed
    (Development|PrintString "hit component")
    (if (Components|ComponentHasTag _hitcomponent "LRED")
      (bind _output_get (Variables|Default|SetCurrentWireIndex 0))
      (if (not (Utilities|Array|Get(acopy) (Variables|Default|GetIsCompleted) _output_get))
        (Utilities|FlowControl|Sequence
          (:then_0
            (Development|PrintString "red")
            (Variables|Default|SetIsDragging true)
            (Development|PrintString "is dragging red true"))
          (:then_1
            (Variables|Default|SetCurrentCable _cable_red))
          (:then_2
            (Variables|Default|SetRequired%20Tag "RRED"))
          (:then_3
            (Rendering|SetVisibility _cable_red true false)
            (Development|PrintString "red cable visible"))
          (:then_4
            (Variables|/Script/CableComponent.CableComponent|SetEndLocation _cable_red "0, 0, 0")
            (Development|PrintString "inil"))))
      (elif (Components|ComponentHasTag _hitcomponent "LBLUE")
        (bind _output_get_2 (Variables|Default|SetCurrentWireIndex 1))
        (if (not (Utilities|Array|Get(acopy) (Variables|Default|GetIsCompleted) _output_get_2))
          (Utilities|FlowControl|Sequence
            (:then_0
              (Variables|Default|SetIsDragging true))
            (:then_1
              (Variables|Default|SetCurrentCable _cable_blue))
            (:then_2
              (Variables|Default|SetRequired%20Tag "RBLUE"))
            (:then_3
              (Rendering|SetVisibility _cable_blue true false))
            (:then_4
              (Variables|/Script/CableComponent.CableComponent|SetEndLocation _cable_blue "0, 0, 0"))))
        (elif (Components|ComponentHasTag _hitcomponent "LYELLOW")
          (bind _output_get_3 (Variables|Default|SetCurrentWireIndex 2))
          (if (not (Utilities|Array|Get(acopy) (Variables|Default|GetIsCompleted) _output_get_3))
            (Utilities|FlowControl|Sequence
              (:then_0
                (Variables|Default|SetIsDragging true))
              (:then_1
                (Variables|Default|SetCurrentCable _cable_yellow))
              (:then_2
                (Variables|Default|SetRequired%20Tag "RYELLOW"))
              (:then_3
                (Rendering|SetVisibility _cable_yellow true false))
              (:then_4
                (Variables|/Script/CableComponent.CableComponent|SetEndLocation _cable_yellow "0, 0, 0"))))
          (elif (Components|ComponentHasTag _hitcomponent "LGREEN")
            (bind _output_get_4 (Variables|Default|SetCurrentWireIndex 3))
            (if (not (Utilities|Array|Get(acopy) (Variables|Default|GetIsCompleted) _output_get_4))
              (Utilities|FlowControl|Sequence
                (:then_0
                  (Variables|Default|SetIsDragging true))
                (:then_1
                  (Variables|Default|SetCurrentCable _cable_green))
                (:then_2
                  (Variables|Default|SetRequired%20Tag "RGREEN"))
                (:then_3
                  (Rendering|SetVisibility _cable_green true false))
                (:then_4
                  (Variables|/Script/CableComponent.CableComponent|SetEndLocation _cable_green "0, 0, 0")))))))))
  (:Released
    (Variables|Default|SetIsDragging false)
    (if (Components|ComponentHasTag _hitcomponent_2 (Variables|Default|GetRequired%20Tag))
      (Variables|/Script/CableComponent.CableComponent|SetEndLocation (Variables|Default|GetCurrentCable) (Math|Transform|InverseTransformLocation (Transformation|GetWorldTransform (Variables|Default|GetCurrentCable)) (Transformation|GetWorldLocation _hitcomponent_2)))
      (Utilities|Array|SetArrayElem (Variables|Default|GetIsCompleted) (Variables|Default|GetCurrentWireIndex) true)
      (else
        (Rendering|SetVisibility (Variables|Default|GetCurrentCable) false false)
        (Variables|Default|SetCurrentCable 0)))))

(fn ConstructionScript)