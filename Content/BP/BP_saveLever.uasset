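; BP_saveLever is a one-shot lever actor that activates a referenced elevator when triggered.
; The first overlap of TriggerBox by any actor sets Used and plays a timeline that rolls the Lever component from zero to LeverPullAngle.
; When the timeline finishes, it calls ActivateElevator on ElevatorRef if valid.
; The play-rate calculation from LeverPullTime is unconnected, so that variable does not affect the pull speed.
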(event OnComponentBeginOverlap(TriggerBox)
  (params (OverlappedComponent :type Primitive%20Component%20Object%20Reference) (OtherActor :type Actor%20Object%20Reference) (OtherComp :type Primitive%20Component%20Object%20Reference) (OtherBodyIndex :type Integer) (bFromSweep :type Boolean) (SweepResult :type Hit%20Result%20Structure%20%28by%20ref%29))
  (bind _elevatorref (Variables|Default|GetElevatorRef))
  (if (not (Variables|Default|GetbUsed))
    (Variables|Default|SetbUsed true)
    (bind _新建轨道_0 (Timeline|TL_LeverPull PlayFromStart)
      (:Update
        (Transformation|SetRelativeRotation (Variables|Default|Getlever) (Math|Rotator|MakeRotator (Math|Float|Lerp 0.0 (Variables|Default|GetLeverPullAngle) _新建轨道_0) 0.0 0.0) false false))
      (:Finished
        (Utilities|IsValid _elevatorref
          (:Is%20Valid
            (Default|ActivateElevator _elevatorref)))))))

(event EventBeginPlay)

(event Collision|EventActorBeginOverlap
  (params (OtherActor :type Actor%20Object%20Reference)))

(event EventTick
  (params (DeltaSeconds :type Float%20%28single-precision%29)))

(fn ConstructionScript)