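; BP_Lever is an interactable lever that the player holds with the left mouse button while inside its trigger box.
; Holding stops player movement and sets LeverState; if BP_Light's State is true, it blends to LeverCamera and runs a timeline to completion state.
; Releasing restores walking and, with that light State true, cancels the timeline, resets state and returns the view.
; Tick prints LeverState for debugging; lever-rotation and elevator-activation logic is unconnected.
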(event OnComponentBeginOverlap(TriggerBox)
  (params (OverlappedComponent :type Primitive%20Component%20Object%20Reference) (OtherActor :type Actor%20Object%20Reference) (OtherComp :type Primitive%20Component%20Object%20Reference) (OtherBodyIndex :type Integer) (bFromSweep :type Boolean) (SweepResult :type Hit%20Result%20Structure%20%28by%20ref%29))
  (Variables|Default|SetisNearLever true))

(event OnComponentEndOverlap(TriggerBox)
  (params (OverlappedComponent :type Primitive%20Component%20Object%20Reference) (OtherActor :type Actor%20Object%20Reference) (OtherComp :type Primitive%20Component%20Object%20Reference) (OtherBodyIndex :type Integer))
  (Variables|Default|SetisNearLever false))

(event EventTick
  (params (DeltaSeconds :type Float%20%28single-precision%29))
  (Development|PrintString (Utilities|String|ToString(Integer) (Variables|Default|GetLeverState))))

(event EventBeginPlay
  (Input|EnableInput (Game|GetPlayerController 0)))

(event Input|MouseEvents|LeftMouseButton
  (params (Key :type Key%20Structure :default "None"))
  (:Pressed
    (bind _asbp_first_person_character (Utilities|Casting|CastToBP_FirstPersonCharacter (Game|GetPlayerCharacter 0)))
    (Variables|Default|SetisHolding true)
    (if (Variables|Default|GetisNearLever)
      (Pawn|Components|CharacterMovement|SetMovementMode (Variables|/Script/Engine.Character|GetCharacterMovement _asbp_first_person_character) "MOVE_None" 0)
      (Variables|Default|SetLeverState 1)
      (bind _returnvalue (Actor|GetActorOfClass "/Game/BP/BP_Light.BP_Light_C"))
      (if (Variables|/Game/BP/BP_Light.BP_Light_C|GetState _returnvalue)
        (bind _returnvalue_2 (Actor|GetActorOfClass "/Game/BP/LeverCamera.LeverCamera_C"))
        (Game|Player|SetViewTargetwithBlend (Game|GetPlayerController 0) _returnvalue_2 1.0 "VTBlend_Linear" 0.0 false)
        (Timeline|时间轴 PlayFromStart
          (:Finished
            (Variables|Default|SetLeverState 2)
            (Utilities|FlowControl|Delay 1.0)
            (bind _asbp_first_person_character_2 (Utilities|Casting|CastToBP_FirstPersonCharacter (Game|GetPlayerCharacter 0)))
            (Game|Player|SetViewTargetwithBlend (Game|GetPlayerController 0) _asbp_first_person_character_2 1.0 "VTBlend_Linear" 0.0 false))))))
  (:Released
    (Pawn|Components|CharacterMovement|SetMovementMode (Variables|/Script/Engine.Character|GetCharacterMovement _asbp_first_person_character) "MOVE_Walking" 0)
    (bind _returnvalue_3 (Actor|GetActorOfClass "/Game/BP/BP_Light.BP_Light_C"))
    (if (Variables|/Game/BP/BP_Light.BP_Light_C|GetState _returnvalue_3)
      (Variables|Default|SetisHolding false)
      (Variables|Default|SetLeverState 0)
      (Utilities|FlowControl|Sequence
        (:then_0
          (Timeline|时间轴 Stop))
        (:then_1
          (bind _asbp_first_person_character_3 (Utilities|Casting|CastToBP_FirstPersonCharacter (Game|GetPlayerCharacter 0)))
          (Game|Player|SetViewTargetwithBlend (Game|GetPlayerController 0) _asbp_first_person_character_3 1.0 "VTBlend_Linear" 0.0 false))))))

(fn ConstructionScript)