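; Signal light actor with red, three orange and green lights that follows the state of the BP_Lever in the level.
; While State is true, Tick polls the lever: 0 resets to red, 1 plays the orange sequence once, 2 shows green and clears State.
; A DoOnce-gated timeline drives the orange intensities, raises the Ball's LED dynamic material "light" parameter, and turns red off after a delay.
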(event EventBeginPlay
  (Rendering|Material|CreateDynamicMaterialInstance (Variables|Default|Getball) 0 "/Game/BP/LED.LED" "ballm" :!class /Script/Engine.PrimitiveComponent))

(event EventTick
  (params (DeltaSeconds :type Float%20%28single-precision%29))
  (bind _orangelight2 (Variables|Default|GetorangeLight2))
  (bind _orangelight1 (Variables|Default|GetorangeLight1))
  (bind _redlight (Variables|Default|GetredLight))
  (bind _orangelight3 (Variables|Default|GetorangeLight3))
  (bind _orangelight2_2 (Variables|Default|GetorangeLight2))
  (bind _orangelight1_2 (Variables|Default|GetorangeLight1))
  (bind _greenlight (Variables|Default|GetgreenLight))
  (bind _redlight_2 (Variables|Default|GetredLight))
  (bind _greenlight_2 (Variables|Default|GetgreenLight))
  (bind _orangelight3_2 (Variables|Default|GetorangeLight3))
  (bind _orangelight2_3 (Variables|Default|GetorangeLight2))
  (bind _redlight_3 (Variables|Default|GetredLight))
  (bind _orangelight1_3 (Variables|Default|GetorangeLight1))
  (bind _orangelight3_3 (Variables|Default|GetorangeLight3))
  (if (Variables|Default|GetState)
    (bind _returnvalue (Actor|GetActorOfClass "/Game/BP/BP_Lever.BP_Lever_C"))
    (switch int (Variables|/Game/BP/BP_Lever.BP_Lever_C|GetLeverState _returnvalue)
      (:Default
        (Rendering|Components|Light|SetIntensity (Variables|Default|GetorangeLight2) 0.0)
        (Rendering|Components|Light|SetIntensity (Variables|Default|GetredLight) 5e+02))
      (:0
        ;[0.15 0.15 0.15 0.5] red
        (Rendering|Components|Light|SetLightColor _redlight "(R=1.000000,G=0.000000,B=0.000000,A=1.000000)" true)
        (Rendering|Components|Light|SetIntensity _redlight 5e+02)
        ;[0.15 0.15 0.15 0.5] orange3
        (Rendering|Components|Light|SetLightColor _orangelight3 "(R=1.000000,G=0.285565,B=0.001034,A=1.000000)" true)
        (Rendering|Components|Light|SetIntensity _orangelight3 0.0)
        ;[0.15 0.15 0.15 0.5] orange2
        (Rendering|Components|Light|SetLightColor _orangelight2_2 "(R=1.000000,G=0.287441,B=0.000911,A=1.000000)" true)
        (Rendering|Components|Light|SetIntensity _orangelight2_2 0.0)
        ;[0.15 0.15 0.15 0.5] orange2
        (Rendering|Components|Light|SetLightColor _orangelight1_2 "(R=1.000000,G=0.287441,B=0.000911,A=1.000000)" true)
        (Rendering|Components|Light|SetIntensity _orangelight1_2 0.0)
        ;[0.15 0.15 0.15 0.5] green
        (Rendering|Components|Light|SetLightColor _greenlight "(R=0.045429,G=1.000000,B=0.001614,A=1.000000)" true)
        (Rendering|Components|Light|SetIntensity _greenlight 0.0)
        (Utilities|FlowControl|Sequence
          (:then_0
            (goto _label Reset))
          (:then_1
            (bind (_direction _新建轨道_0 _新建轨道_1 _新建轨道_2) (Timeline|时间轴 Stop)
              (:Update
                (Utilities|FlowControl|Sequence
                  (:then_0
                    ;[0.15 0.15 0.15 0.5] orange1
                    (Rendering|Components|Light|SetLightColor _orangelight1_3 "(R=1.000000,G=0.287441,B=0.000911,A=1.000000)" true)
                    (Rendering|Components|Light|SetIntensity _orangelight1_3 _新建轨道_0)
                    (Rendering|Material|SetScalarParameterValueonMaterials (Variables|Default|Getball) "light" 1e+02)
                    ;[0.15 0.15 0.15 0.5] orange2
                    (Rendering|Components|Light|SetLightColor _orangelight2_3 "(R=1.000000,G=0.287441,B=0.000911,A=1.000000)" true)
                    (Rendering|Components|Light|SetIntensity _orangelight2_3 _新建轨道_1)
                    ;[0.15 0.15 0.15 0.5] orange3
                    (Rendering|Components|Light|SetLightColor _orangelight3_2 "(R=1.000000,G=0.287441,B=0.000911,A=1.000000)" true)
                    (Rendering|Components|Light|SetIntensity _orangelight3_2 _新建轨道_2))
                  (:then_1
                    (Utilities|FlowControl|Delay 1.9)
                    ;;[0.15 0.15 0.15 0.5] red
                    (Rendering|Components|Light|SetLightColor _redlight_2 "(R=1.000000,G=0.000000,B=0.000000,A=1.000000)" true)
                    (Rendering|Components|Light|SetIntensity _redlight_2 0.0))))))))
      (:1
        (Utilities|FlowControl|DoOnce false :!label _label
          (:Completed
            (Timeline|时间轴 PlayFromStart))))
      (:2
        ;[0.15 0.15 0.15 0.5] red
        (Rendering|Components|Light|SetLightColor _redlight_3 "(R=1.000000,G=0.000000,B=0.000000,A=1.000000)" true)
        (Rendering|Components|Light|SetIntensity _redlight_3 0.0)
        ;[0.15 0.15 0.15 0.5] orange3
        (Rendering|Components|Light|SetLightColor _orangelight3_3 "(R=1.000000,G=0.285565,B=0.001034,A=1.000000)" true)
        (Rendering|Components|Light|SetIntensity _orangelight3_3 0.0)
        ;[0.15 0.15 0.15 0.5] orange2
        (Rendering|Components|Light|SetLightColor _orangelight2 "(R=1.000000,G=0.287441,B=0.000911,A=1.000000)" true)
        (Rendering|Components|Light|SetIntensity _orangelight2 0.0)
        ;[0.15 0.15 0.15 0.5] orange2
        (Rendering|Components|Light|SetLightColor _orangelight1 "(R=1.000000,G=0.287441,B=0.000911,A=1.000000)" true)
        (Rendering|Components|Light|SetIntensity _orangelight1 0.0)
        ;[0.15 0.15 0.15 0.5] green
        (Rendering|Components|Light|SetLightColor _greenlight_2 "(R=0.045429,G=1.000000,B=0.001614,A=1.000000)" true)
        (Rendering|Components|Light|SetIntensity _greenlight_2 5e+02)
        (Utilities|FlowControl|Sequence
          (:then_0
            (Timeline|时间轴 Stop))
          (:then_1
            (Variables|Default|SetState false)))))))

(fn ConstructionScript)