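; Ambient emitter actor that plays occasional one-shot metal rattle and rushing wind sounds at its own location.
; From BeginPlay it loops indefinitely, waiting a random 10 to 20 seconds before each sound.
; Two nested random booleans pick one of four sounds with equal odds, played at the root component's world location, then execution wires back into the delay.
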(event EventBeginPlay
  (bind _self self)
  (bind _defaultsceneroot (Variables|Default|GetDefaultSceneRoot _self))
  (bind _returnvalue (Transformation|GetWorldLocation _defaultsceneroot))
  (Utilities|FlowControl|Delay (Math|Random|RandomFloatinRange 1e+01 2e+01) :!label _label)
  ;[0.15 0.15 0.15 0.5] Randomiser 1
  (if (Math|Random|RandomBool)
    ;[0.15 0.15 0.15 0.5] Randomiser 2
    (if (Math|Random|RandomBool)
      ;[0.15 0.15 0.15 0.5] Sounds
      (Audio|PlaySoundatLocation "/Game/Audio/AmbientSounds/Metal_Rattles.Metal_Rattles" _returnvalue "0, 0, 0" 1.0 1.0 0.0 0 0 0 0)
      (goto _label)
      (else
        (Audio|PlaySoundatLocation "/Game/Audio/AmbientSounds/Metal_Rattles_2.Metal_Rattles_2" _returnvalue "0, 0, 0" 1.0 1.0 0.0 0 0 0 0)
        (goto _label)))
    (else
      ;[0.15 0.15 0.15 0.5] Randomiser 2
      (if (Math|Random|RandomBool)
        (Audio|PlaySoundatLocation "/Game/Audio/AmbientSounds/Wind_Rushing.Wind_Rushing" _returnvalue "0, 0, 0" 1.0 1.0 0.0 0 0 0 0)
        (goto _label)
        (else
          (Audio|PlaySoundatLocation "/Game/Audio/AmbientSounds/Wind_Rushing_2.Wind_Rushing_2" _returnvalue "0, 0, 0" 1.0 1.0 0.0 0 0 0 0)
          (goto _label))))))

(event Collision|EventActorBeginOverlap
  (params (OtherActor :type Actor%20Object%20Reference)))

(event EventTick
  (params (DeltaSeconds :type Float%20%28single-precision%29)))

(fn ConstructionScript)