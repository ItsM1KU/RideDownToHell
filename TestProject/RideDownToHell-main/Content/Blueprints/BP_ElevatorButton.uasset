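; BP_ElevatorButton is an interactable elevator button that closes its referenced door when the player interacts with it.
; Interact calls CloseDoor on DoorReference.
; OnFocus and NotonFocus toggle an outline overlay material on ButtonMesh to show when the button is targeted.
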(event EventBeginPlay
  (|CallParentFunction) ; This node is disabled and will not be called.\nDrag off pins to build functionality.
)

(event Collision|EventActorBeginOverlap
  (params (OtherActor :type Actor%20Object%20Reference))
  (|CallParentFunction OtherActor) ; This node is disabled and will not be called.\nDrag off pins to build functionality.
)

(event EventTick
  (params (DeltaSeconds :type Float%20%28single-precision%29))
  (|CallParentFunction DeltaSeconds) ; This node is disabled and will not be called.\nDrag off pins to build functionality.
)

(event EventOnFocus
  (Rendering|Material|SetOverlayMaterial (Variables|Default|GetButtonMesh) "/Game/LevelPrototyping/Materials/M_InteractOutline.M_InteractOutline" :!class /Script/Engine.MeshComponent))

(event EventNotonFocus
  (Rendering|Material|SetOverlayMaterial (Variables|Default|GetButtonMesh) 0 :!class /Script/Engine.MeshComponent))

(event EventInteract
  (Default|CloseDoor (Variables|Default|GetDoorReference)))

(fn ConstructionScript
  (|CallParentFunction))